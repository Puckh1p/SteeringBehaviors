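; Actor that implements a flee steering behavior, moving its construction-script static mesh away from nearby target actors.
; BeginPlay gathers all actors of the Target classes into FleeTarget.
; Tick loops over them when MultiplesObstacles is set, otherwise running one distance check without iterating.
; Within EffectMinimumDistance, it interpolates rotation away using a look-at between negated locations and moves along local X by Velocity after a one-frame Delay.
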(event EventBeginPlay
  (for _array_element (Variables|Flee|GetTarget)
    (bind _outactors (Actor|GetAllActorsOfClass _array_element))
    (for _array_element_2 _outactors
      (Utilities|Array|Add (Variables|Default|GetFleeTarget) _array_element_2))))

(event EventTick
  (params (DeltaSeconds :type Float%20%28single-precision%29))
  (if (Variables|Flee|GetMultiplesObstacles)
    (for (_array_element _array_index) (Variables|Default|GetFleeTarget)
      ;[1 1 1] Defines a minimum distance between Static Mesh and Target
      (if (< (Transformation|GetDistanceTo _array_element) (Variables|Flee|GetEffectMinimumDistance))
        (Utilities|FlowControl|Sequence
          (:then_0
            ;[1 1 1] This sets the Static Mesh to move 5 units forward
            (Utilities|FlowControl|Delay (Utilities|Time|GetWorldDeltaSeconds))
            (Transformation|AddActorLocalOffset (Math|Vector|MakeVector (Variables|Flee|GetVelocity) 0.0 0.0) false false))
          (:then_1
            ;[1 1 1] Set the Static Mesh to rotate based on the target's opposite location
            (Transformation|SetActorRotation (Math|Interpolation|RInterpTo (Transformation|GetActorRotation) (Math|Rotator|FindLookatRotation (Math|Vector|NegateVector (Transformation|GetActorLocation)) (Math|Vector|NegateVector (Transformation|GetActorLocation (Utilities|Array|Get(acopy) (Variables|Default|GetFleeTarget) _array_index)))) (Utilities|Time|GetWorldDeltaSeconds) 5.0))))))
    (else
      (if (< (Transformation|GetDistanceTo _array_element) (Variables|Flee|GetEffectMinimumDistance))
        (Utilities|FlowControl|Sequence
          (:then_0
            (Utilities|FlowControl|Delay (Utilities|Time|GetWorldDeltaSeconds))
            (Transformation|AddActorLocalOffset (Math|Vector|MakeVector (Variables|Flee|GetVelocity) 0.0 0.0) false false))
          (:then_1
            (Transformation|SetActorRotation (Math|Interpolation|RInterpTo (Transformation|GetActorRotation) (Math|Rotator|FindLookatRotation (Math|Vector|NegateVector (Transformation|GetActorLocation)) (Math|Vector|NegateVector (Transformation|GetActorLocation (Utilities|Array|Get(acopy) (Variables|Default|GetFleeTarget) _array_index)))) (Utilities|Time|GetWorldDeltaSeconds) 5.0))))))))

(fn ConstructionScript
  (bind _returnvalue (AddComponent|AddStaticMeshComponent false (Math|Transform|MakeTransform "0, 0,-50.000000" "0, 0, 0" "1.000000,1.000000,1.000000")))
  (Components|StaticMesh|SetStaticMesh _returnvalue (Variables|Flee|GetStaticMesh)))