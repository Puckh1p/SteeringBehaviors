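; BP_Seek is a steering-behavior actor that moves forward constantly while turning toward a target.
; On BeginPlay it gathers all actors of the Target classes into SeekTarget.
; Each Tick it advances along local X by an unscaled Velocity, smoothly rotates toward the minimum-distance entry, then refreshes distances only when ClosestTarget is set.
; The construction script adds the configurable static mesh.
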(event EventBeginPlay
  (for _array_element (Variables|Seek|GetTarget)
    (bind _outactors (Actor|GetAllActorsOfClass _array_element))
    (for _array_element_2 _outactors
      (Utilities|Array|Add (Variables|Default|GetSeekTarget) _array_element_2))))

(event EventTick
  (params (DeltaSeconds :type Float%20%28single-precision%29))
  (Utilities|FlowControl|Sequence
    (:then_0
      ;[1 1 1] Set la static mesh para que avance
      (Transformation|AddActorLocalOffset (Math|Vector|MakeVector (Variables|Seek|GetVelocity) 0.0 0.0) false false))
    (:then_1
      ;[1 1 1] Esto set para que gire la static mesh según la ubicacion del target
      (Transformation|SetActorRotation (Math|Interpolation|RInterpTo (Transformation|GetActorRotation) (Math|Rotator|FindLookatRotation (Transformation|GetActorLocation) (Transformation|GetActorLocation (Utilities|Array|Get(acopy) (Variables|Default|GetSeekTarget) (.IndexOfMinValue (Math|Float|MinOfFloatArray (Variables|Default|GetTargetDistance)))))) (Utilities|Time|GetWorldDeltaSeconds) 5.0)))
    (:then_2
      ;[1 1 1] Almacena la distancia entre el target y el actor
      (if (Variables|Seek|GetClosestTarget)
        (for (_array_element _array_index) (Variables|Default|GetSeekTarget)
          (Utilities|Array|SetArrayElem (Variables|Default|GetTargetDistance) _array_index (Transformation|GetDistanceTo _array_element) true))))))

(fn ConstructionScript
  (bind _returnvalue (AddComponent|AddStaticMeshComponent false (Math|Transform|MakeTransform "0, 0,-50.000000" "0, 0, 0" "1.000000,1.000000,1.000000")))
  (Components|StaticMesh|SetStaticMesh _returnvalue (Variables|Seek|GetStaticMesh)))