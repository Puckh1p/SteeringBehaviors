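; Steering-behavior pursuit actor that chases actors of the configured target classes, gathered on BeginPlay.
; Each tick it moves along its local X axis by Velocity and, when ClosestTarget is set, records every target's distance.
; Distance checks scale Velocity down or zero it near targets, never restoring it.
; It smoothly rotates toward a point projected ahead of the target with the smallest stored distance, along that target's forward vector.
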(event EventBeginPlay
  (for _array_element (Variables|Pursuit|GetTarget)
    (bind _outactors (Actor|GetAllActorsOfClass _array_element))
    (for _array_element_2 _outactors
      (Utilities|Array|Add (Variables|Default|GetPursuitTarget) _array_element_2))))

(event EventTick
  (params (DeltaSeconds :type Float%20%28single-precision%29))
  (bind _pursuittarget (Variables|Default|GetPursuitTarget))
  (bind _targetdistance (Variables|Default|GetTargetDistance))
  (bind _indexofminvalue (Math|Float|MinOfFloatArray _targetdistance))
  (bind _output (Utilities|Array|Get(acopy) _pursuittarget _indexofminvalue))
  (Utilities|FlowControl|Sequence
    (:then_0
      ;[1 1 1] Esto configura la static mesh para que avance
      (Transformation|AddActorLocalOffset (Math|Vector|MakeVector (Variables|Pursuit|GetVelocity) 0.0 0.0) false false))
    (:then_1
      (if (Variables|Pursuit|GetClosestTarget)
        (for (_array_element _array_index) (Variables|Default|GetPursuitTarget)
          ;[1 1 1] Almacena la distancia entre el actor y el target
          (Utilities|Array|SetArrayElem (Variables|Default|GetTargetDistance) _array_index (Transformation|GetDistanceTo _array_element) true)
          ;[1 1 1] Set una distancia minima entre la static mesh y el target para iniciar una desaceleracion
          (if (> (Transformation|GetDistanceTo _array_element) (Variables|Default|GetDecelerationMinimumDistance)) ; Si la distancia llega a ser mayor a 1000, la static mesh no se relentiza, pero si es inferior a 1000, se inicia el segundo branch.
            (Variables|Pursuit|SetVelocity (Variables|Pursuit|GetVelocity))
            (elif (> (Transformation|GetDistanceTo _array_element) (Variables|Default|GetStopMinimumDistance)) ; Si la distancia está entre 1000 y 150, la static mesh desacelera según la distancia. Si la distancia es menor a 120 el target deja de moverse.
              (Variables|Pursuit|SetVelocity (/ (Transformation|GetDistanceTo _array_element) (Variables|Default|GetDecelerationIntensity)))
              (else
                (Variables|Pursuit|SetVelocity 0.0)))))
        (else
          (if (> (Transformation|GetDistanceTo _array_element) (Variables|Default|GetDecelerationMinimumDistance)) ; Si la distancia llega a ser mayor a 1000, la static mesh no se relentiza, pero si es inferior a 1000, se inicia el segundo branch.
            (Variables|Pursuit|SetVelocity (Variables|Pursuit|GetVelocity))
            (elif (> (Transformation|GetDistanceTo _array_element) (Variables|Default|GetStopMinimumDistance)) ; Si la distancia está entre 1000 y 150, la static mesh desacelera según la distancia. Si la distancia es menor a 120 el target deja de moverse.
              (Variables|Pursuit|SetVelocity (/ (Transformation|GetDistanceTo _array_element) (Variables|Default|GetDecelerationIntensity)))
              (else
                (Variables|Pursuit|SetVelocity 0.0)))))))
    (:then_2
      ;[1 1 1] Esto set la static mesh para que gire según la ubicacion del target
      (Transformation|SetActorRotation (Math|Interpolation|RInterpTo (Transformation|GetActorRotation) (Math|Rotator|FindLookatRotation (Transformation|GetActorLocation) (+ (Transformation|GetActorLocation _output) (* (Transformation|GetActorForwardVector _output) (Variables|Pursuit|GetTargetForwardDistance)))) (Utilities|Time|GetWorldDeltaSeconds) 5.0)))))

(fn ConstructionScript
  (bind _returnvalue (AddComponent|AddStaticMeshComponent false (Math|Transform|MakeTransform "0, 0,-50.000000" "0, 0, 0" "1.000000,1.000000,1.000000")))
  (Components|StaticMesh|SetStaticMesh _returnvalue (Variables|Pursuit|GetStaticMesh)))