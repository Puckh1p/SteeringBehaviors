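; BP_Leader is a steering-behavior actor that moves forward and performs an arrival behavior toward target actors.
; BeginPlay gathers all actors of the configured classes, and the construction script adds its static mesh.
; Each Tick offsets it by Velocity, reducing that with target distance to a stop, and smoothly rotates it toward the target with the smallest recorded distance.
; The ClosestTarget flag gates the loop that records those distances.
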(event EventBeginPlay
  (for _array_element (Variables|Leader|GetTarget)
    (bind _outactors (Actor|GetAllActorsOfClass _array_element))
    (for _array_element_2 _outactors
      (Utilities|Array|Add (Variables|Default|GetArrivalTarget) _array_element_2))))

(event EventTick
  (params (DeltaSeconds :type Float%20%28single-precision%29))
  (Utilities|FlowControl|Sequence
    (:then_0
      ;[1 1 1] This sets the Static Mesh to move 5 units forward
      (Transformation|AddActorLocalOffset (Math|Vector|MakeVector (Variables|Leader|GetVelocity) 0.0 0.0) false false))
    (:then_1
      (if (Variables|Leader|GetClosestTarget)
        (for (_array_element _array_index) (Variables|Default|GetArrivalTarget)
          ;[1 1 1] Stores the distances between the Actor and the Targets
          (Utilities|Array|SetArrayElem (Variables|Default|GetArrivalDistance) _array_index (Transformation|GetDistanceTo _array_element) true)
          ;[1 1 1] Set a minimum distance between the Static Mesh and the Target to initiate a deceleration
          (if (> (Transformation|GetDistanceTo _array_element) (Variables|Leader|GetDecelerationMinimumDistance)) ; (1st Check) If the distance is greater than 1000 units, the Static Mesh does not slow down. If the distance is less than 1000 units, the 2nd Verification will start.
            _
            (elif (> (Transformation|GetDistanceTo _array_element) (Variables|Leader|GetStopMinimumDistance)) ; (2nd Check) If the distance is between 1000 and 150 units, the Static Mesh decelerates based on the distance. If the distance is less than 120 the cube stops moving.
              (Variables|Leader|SetVelocity (/ (Transformation|GetDistanceTo _array_element) (Variables|Leader|GetDecelerationIntensity)))
              (else
                (Variables|Leader|SetVelocity 0.0))))
          ;[1 1 1] Set the Static Mesh to rotate based on the Target's location
          (Transformation|SetActorRotation (Math|Interpolation|RInterpTo (Transformation|GetActorRotation) (Math|Rotator|FindLookatRotation (Transformation|GetActorLocation) (Transformation|GetActorLocation (Utilities|Array|Get(acopy) (Variables|Default|GetArrivalTarget) (.IndexOfMinValue (Math|Float|MinOfFloatArray (Variables|Default|GetArrivalDistance)))))) (Utilities|Time|GetWorldDeltaSeconds) 5.0)))
        (else
          (if (> (Transformation|GetDistanceTo _array_element) (Variables|Leader|GetDecelerationMinimumDistance)) ; (1st Check) If the distance is greater than 1000 units, the Static Mesh does not slow down. If the distance is less than 1000 units, the 2nd Verification will start.
            _
            (elif (> (Transformation|GetDistanceTo _array_element) (Variables|Leader|GetStopMinimumDistance)) ; (2nd Check) If the distance is between 1000 and 150 units, the Static Mesh decelerates based on the distance. If the distance is less than 120 the cube stops moving.
              (Variables|Leader|SetVelocity (/ (Transformation|GetDistanceTo _array_element) (Variables|Leader|GetDecelerationIntensity)))
              (else
                (Variables|Leader|SetVelocity 0.0))))
          (Transformation|SetActorRotation (Math|Interpolation|RInterpTo (Transformation|GetActorRotation) (Math|Rotator|FindLookatRotation (Transformation|GetActorLocation) (Transformation|GetActorLocation (Utilities|Array|Get(acopy) (Variables|Default|GetArrivalTarget) (.IndexOfMinValue (Math|Float|MinOfFloatArray (Variables|Default|GetArrivalDistance)))))) (Utilities|Time|GetWorldDeltaSeconds) 5.0)))))))

(fn ConstructionScript
  (bind _returnvalue (AddComponent|AddStaticMeshComponent false (Math|Transform|MakeTransform "0, 0,-50.000000" "0, 0, 0" "1.000000,1.000000,1.000000")))
  (Components|StaticMesh|SetStaticMesh _returnvalue (Variables|Leader|GetStaticMesh)))