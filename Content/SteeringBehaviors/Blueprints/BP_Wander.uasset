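; Wandering actor that roams between random points in a box around a fixed world-space center near the origin.
; Each tick it moves forward by Velocity, without delta-time scaling, while RInterpTo eases its rotation toward the destination.
; Within 100 units it either stops (Wait) or picks a new point; farther away, a Delay of NewDirectionTime triggers re-picking.
; The construction script adds its configurable static mesh.
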(event EventBeginPlay
  ;[1 1 1] Choose a random point when Actor play.
  (Variables|Default|SetNewDestination (Math|Random|RandomPointinBoundingBox "0, 0,50.000000" (Math|Vector|MakeVector (Variables|Wander|GetMaxBoxExtentX) (Variables|Wander|GetMaxBoxExtentY) (Variables|Wander|GetMaxBoxExtentZ)))))

(event EventTick
  (params (DeltaSeconds :type Float%20%28single-precision%29))
  (Utilities|FlowControl|Sequence
    (:then_0
      ;[1 1 1] This sets the Static Mesh to move 5 units forward
      (Transformation|AddActorLocalOffset (Math|Vector|MakeVector (Variables|Wander|GetVelocity) 0.0 0.0) false false))
    (:then_1
      ;[1 1 1] This sets the static mesh to rotate based on the value of the New Destination variable
      (Transformation|SetActorRotation (Math|Interpolation|RInterpTo (Transformation|GetActorRotation) (Math|Rotator|FindLookatRotation (Transformation|GetActorLocation) (Variables|Default|GetNewDestination)) (Utilities|Time|GetWorldDeltaSeconds) 5.0)))
    (:then_2
      ;[1 1 1] Set, every 2 sec, the value of the New Destination variable based on a random point
      (if (<= (Math|Vector|Distance(Vector) (Transformation|GetActorLocation) (Variables|Default|GetNewDestination)) 1e+02)
        (if (Variables|Wander|GetWait)
          (Variables|Wander|SetVelocity 0.0)
          (else
            (Variables|Default|SetNewDestination (Math|Random|RandomPointinBoundingBox "0, 0,50.000000" (Math|Vector|MakeVector (Variables|Wander|GetMaxBoxExtentX) (Variables|Wander|GetMaxBoxExtentY) (Variables|Wander|GetMaxBoxExtentZ))) :!label _label)
            (Variables|Wander|SetVelocity 1e+01)))
        (else
          (Utilities|FlowControl|Delay (Variables|Wander|GetNewDirectionTime))
          (goto _label))))))

(fn ConstructionScript
  (bind _returnvalue (AddComponent|AddStaticMeshComponent false (Math|Transform|MakeTransform "0, 0,-50.000000" "0, 0, 0" "1.000000,1.000000,1.000000")))
  (Components|StaticMesh|SetStaticMesh _returnvalue (Variables|Wander|GetStaticMesh)))